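; BP_Player is the player character, handling movement, jump, sprint, crouch and interaction through Enhanced Input actions, and creating the main HUD on BeginPlay.
; Sprint and crouch change max walk speed, with sprint starting only while moving and crouch also blending capsule half-height through a reversible timeline.
; Interact line-traces forward from the camera and sends InteractMessage to hit actors implementing BPI_Interaction.
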(event Input|EnhancedActionEvents|EnhancedInputActionIA_Move
  (params (ActionValue :type Vector%202D%20Structure) (ElapsedSeconds :type Float%20%28double-precision%29) (TriggeredSeconds :type Float%20%28double-precision%29) (InputAction :type Input%20Action%20Object%20Reference :default "/Game/Player/Input/Actions/IA_Move.IA_Move"))
  (Utilities|FlowControl|Sequence
    (:then_0
      (Pawn|Input|AddMovementInput (Transformation|GetActorRightVector) (.x ActionValue) false))
    (:then_1
      (Pawn|Input|AddMovementInput (Transformation|GetActorForwardVector) (.y ActionValue) false))))

(event Input|EnhancedActionEvents|EnhancedInputActionIA_Crouch
  (params (ActionValue :type Boolean) (ElapsedSeconds :type Float%20%28double-precision%29) (TriggeredSeconds :type Float%20%28double-precision%29) (InputAction :type Input%20Action%20Object%20Reference :default "/Game/Player/Input/Actions/IA_Crouch.IA_Crouch"))
  (bind _charactermovement (Variables|Character|GetCharacterMovement))
  (:Triggered
    (Variables|/Script/Engine.CharacterMovementComponent|SetMaxWalkSpeed _charactermovement 3e+02)
    (bind _crouch (Timeline|Timeline_Crouch Play)
      (:Update
        (Components|Capsule|SetCapsuleHalfHeight (Variables|Collision|GetCapsuleComponent) (Math|Float|Lerp 88.0 4e+01 _crouch) true))))
  (:Completed
    (Variables|/Script/Engine.CharacterMovementComponent|SetMaxWalkSpeed _charactermovement 4e+02)
    (Timeline|Timeline_Crouch Reverse)))

(event Input|EnhancedActionEvents|EnhancedInputActionIA_Interact
  (params (ActionValue :type Boolean) (ElapsedSeconds :type Float%20%28double-precision%29) (TriggeredSeconds :type Float%20%28double-precision%29) (InputAction :type Input%20Action%20Object%20Reference :default "/Game/Player/Input/Actions/IA_Interact.IA_Interact"))
  (:Completed
    (bind _hitactor (CallFunction|LineTrace 3.5e+02))
    (if (and (Utilities|IsValid _hitactor) (Utilities|DoesObjectImplementInterface _hitactor "/Game/Player/Input/Interfaces/BPI_Interaction.BPI_Interaction_C"))
      (Class|BPIInteraction|Interact(Message) _hitactor))))

(event Input|EnhancedActionEvents|EnhancedInputActionIA_Jump
  (params (ActionValue :type Boolean) (ElapsedSeconds :type Float%20%28double-precision%29) (TriggeredSeconds :type Float%20%28double-precision%29) (InputAction :type Input%20Action%20Object%20Reference :default "/Game/Player/Input/Actions/IA_Jump.IA_Jump"))
  (:Triggered
    (Character|Jump))
  (:Completed
    (Character|StopJumping)))

(event Input|EnhancedActionEvents|EnhancedInputActionIA_Sprint
  (params (ActionValue :type Boolean) (ElapsedSeconds :type Float%20%28double-precision%29) (TriggeredSeconds :type Float%20%28double-precision%29) (InputAction :type Input%20Action%20Object%20Reference :default "/Game/Player/Input/Actions/IA_Sprint.IA_Sprint"))
  (:Triggered
    (if (Utilities|Operators|NotEqual(!=) :A (Transformation|GetVelocity))
      (CallFunction|StartSprint)))
  (:Completed
    (CallFunction|StopSprint)))

(event EventBeginPlay
  (CallFunction|Initialize))

(event Collision|EventActorBeginOverlap
  (params (OtherActor :type Actor%20Object%20Reference)))

(event EventTick
  (params (DeltaSeconds :type Float%20%28single-precision%29)))

(fn ConstructionScript)

(fn StartSprint
  (Variables|/Script/Engine.CharacterMovementComponent|SetMaxWalkSpeed (Variables|Character|GetCharacterMovement) 8e+02))

(fn StopSprint
  (Variables|/Script/Engine.CharacterMovementComponent|SetMaxWalkSpeed (Variables|Character|GetCharacterMovement) 4e+02))

(fn LineTrace
  (params (Length :type Float%20%28double-precision%29))
  (bind _camera (Variables|Default|GetCamera))
  (bind _returnvalue (Transformation|GetWorldLocation _camera))
  (bind _outhit (Collision|LineTraceByChannel _returnvalue (+ _returnvalue (* (Math|Vector|GetForwardVector _camera) Length)) "TraceTypeQuery1" false 0 "None"))
  (return (.HitActor (Collision|BreakHitResult _outhit))))

(fn Initialize
  (bind _returnvalue (UserInterface|CreateWidget "/Game/HUD/W_MainHUD.W_MainHUD_C"))
  (bind _output_get (Variables|Default|SetMainHUDRef _returnvalue))
  (UserInterface|Viewport|AddtoViewport _output_get 0))