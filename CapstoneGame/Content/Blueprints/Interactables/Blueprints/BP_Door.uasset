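; BP_Door is an interactable hinged door that swings open away from or toward a side chosen by the player's position.
; On Interact it toggles a closed flag and plays a timeline forward to open or reverses it from the end to close.
; The dot product of the player-to-door direction and the door's forward vector picks the sign of the 90-degree yaw applied to the Door component.
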(event EventBeginPlay
  (|CallParentFunction) ; This node is disabled and will not be called.\nDrag off pins to build functionality.
)

(event Collision|EventActorBeginOverlap
  (params (OtherActor :type Actor%20Object%20Reference))
  (|CallParentFunction OtherActor) ; This node is disabled and will not be called.\nDrag off pins to build functionality.
)

(event EventTick
  (params (DeltaSeconds :type Float%20%28single-precision%29))
  (|CallParentFunction DeltaSeconds) ; This node is disabled and will not be called.\nDrag off pins to build functionality.
)

(event EventInteract
  (bind _self self)
  (if (Variables|Default|GetIsDoorClosed)
    (Variables|Default|SetIsDoorClosed false)
    (Variables|Default|SetDotProduct (Math|Vector|DotProduct (Math|Vector|Normalize (- (Transformation|GetActorLocation _self) (Transformation|GetActorLocation (Variables|Default|GetPlayerRef)))) (Transformation|GetActorForwardVector _self)))
    (bind _door (Timeline|Timeline_Door Play)
      (:Update
        (Transformation|SetRelativeRotation (Variables|Default|GetDoor) (Math|Rotator|MakeRotator 0.0 0.0 (Math|Float|Lerp 0.0 (select (>= (Variables|Default|GetDotProduct) 0.0) 9e+01 -9e+01) _door)) false false)))
    (else
      (Variables|Default|SetIsDoorClosed true)
      (Timeline|Timeline_Door ReverseFromEnd))))

(fn ConstructionScript
  (|CallParentFunction))